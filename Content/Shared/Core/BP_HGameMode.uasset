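; BP_HGameMode is a shared game mode Blueprint that configures the player's audio listener and draws its debug view every tick.
; SetupAudioListenerBP either clears the listener overrides or, when enabled with a tag, finds the first matching scene component on the controlled pawn.
; It then splits the listener, attaching attenuation to that component while position and orientation follow the camera manager's transform.
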(event `self.ReceiveTick`
  (params (DeltaSeconds :type "Float (single-precision)"))
  (`self.DrawAudioListenerDebugCPP`))

(fn `SetupAudioListenerBP`
  (params (PlayerController :type "PlayerController Object Reference") (OverrideAttenuation :type Boolean) (AttenuationComponentTag :type Name :default "AttenuationOverride"))
  (bind _playercontroller (`local.PlayerController`))
  (bind _returnvalue (`self.GetComponentsByTag` (`Controller.K2_GetPawn` (`local.PlayerController`)) "/Script/Engine.SceneComponent" (`local.AttenuationComponentTag`)))
  (`/Engine/EditorBlueprintResources/StandardMacros.IsValid` PlayerController
    (:`Is Valid`
      (if (or (not (`local.OverrideAttenuation`)) (== (`local.AttenuationComponentTag`) "None"))
        (`PlayerController.ClearAudioListenerAttenuationOverride` _playercontroller)
        (`PlayerController.ClearAudioListenerOverride` _playercontroller)
        (elif (`KismetArrayLibrary.Array_IsNotEmpty` _returnvalue)
          (`PlayerController.SetAudioListenerAttenuationOverride` (`local.PlayerController`) (`|GetArrayItem` _returnvalue) (0.0 0.0 0.0))
          (`PlayerController.SetAudioListenerOverride` :`self` (`local.PlayerController`) :`AttachToComponent` (`PlayerCameraManager.TransformComponent` (`PlayerController.PlayerCameraManager` (`local.PlayerController`)))))))))

(fn `UserConstructionScript`)